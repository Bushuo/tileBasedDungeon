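; BasicRangedAttack is a projectile Blueprint that plays a particle effect when its lifecycle ends.
; Its EndLifecycle override zeroes Speed and spawns the DamageFromProjectile emitter at the actor's location.
; The parent EndLifecycle is deferred until that particle system reports it has finished.
; An older Pawn-filtered copy of this sequence is left disconnected, and the overlap event does nothing.
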(event `self.EndLifecycle`
  (set `self.speed_` 0.0)
  (bind _returnvalue (`GameplayStatics.SpawnEmitterAtLocation` "/Game/Effects/DamageFromProjectile.DamageFromProjectile" (`self.K2_GetActorLocation`)))
  (add `ParticleSystemComponent.OnSystemFinished` _returnvalue (delegate `FinishedPlayingParticle`)))

(event `FinishedPlayingParticle`
  (params (PSystem :type "ParticleSystemComponent Object Reference"))
  (`parent.EndLifecycle`))

(event `self.ReceiveActorBeginOverlap`
  (params (OtherActor :type "Actor Object Reference"))
  ;[1 1 1] On Actor Overlap
)

(fn `UserConstructionScript`)