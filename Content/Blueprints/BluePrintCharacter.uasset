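; Top-down player character Blueprint that moves along world axes, turns to face the cursor and fires a mage basic-attack projectile.
; BeginPlay adds the DungeonHUD widget to the viewport.
; The attack uses a busy flag and two Delays, split by AttackSpeed, for wind-up and cooldown around the spawn.
; Tick caps Health at one, regenerates it through a Delay, and yaws the capsule toward the cursor hit point.
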(event `InputAxis|MoveStraight`
  (params (AxisValue :type "Float (single-precision)"))
  ;[1 1 1] Movement
  (`self.AddMovementInput` (1.0 0.0 0.0) AxisValue))

(event `InputAxis|MoveSideways`
  (params (AxisValue :type "Float (single-precision)"))
  ;[1 1 1] Movement
  (`self.AddMovementInput` (0.0 1.0 0.0) AxisValue))

(event `self.ReceiveBeginPlay`
  ;[1 1 1] Display HUD
  (bind _returnvalue (`|CreateWidget` "/Game/Blueprints/DungeonHUD.DungeonHUD_C"))
  (`UserWidget.AddToViewport` _returnvalue 0))

(event `InputAction|BasicAttack`
  (params (Key :type "Key Structure"))
  (bind _attackspeed (`self.AttackSpeed`))
  ;[1 1 1] Basic Attack
  (:`Pressed`
    (if (not (`self.BasickAttacking`))
      (set `self.BasickAttacking` true)
      (`KismetSystemLibrary.Delay` _attackspeed)
      (`|SpawnActorFromClass` "/Game/Blueprints/Projectile_MageBAtk.Projectile_MageBAtk_C" (`KismetMathLibrary.MakeTransform` (+ (.location (`self.GetTransform`)) (0.0 0.0 35.0)) (.rotation (`self.GetTransform`)) (.scale (`self.GetTransform`))) "Undefined" "OverrideRootScale" null null)
      (`KismetSystemLibrary.Delay` (- 1.5 _attackspeed))
      (set `self.BasickAttacking` false))))

(event `self.ReceiveTick`
  (params (DeltaSeconds :type "Float (single-precision)"))
  (bind (_returnvalue_roll _returnvalue_pitch) (`KismetMathLibrary.BreakRotator` (`self.K2_GetActorRotation`)))
  (bind (_returnvalue_roll_2 _returnvalue_pitch_2 _returnvalue_yaw) (`KismetMathLibrary.BreakRotator` (`KismetMathLibrary.FindLookAtRotation` (`self.K2_GetActorLocation`) (`.Location` (`GameplayStatics.BreakHitResult` (`PlayerController.GetHitResultUnderCursorByChannel` (`GameplayStatics.GetPlayerController` 0) "TraceTypeQuery1" false))))))
  (`|ExecutionSequence`
    (:`then_0`
      ;[1 1 1] Reset each tick
      (if (> (`self.Health`) 1.0)
        (set `self.Health` 1.0)))
    (:`then_1`
      ;[1 1 1] Health Regeneration
      (if (< (`self.Health`) 1.0)
        (`KismetSystemLibrary.Delay` 1.0)
        (set `self.Health` (+ (`self.Health`) (* (`self.Regeneration Value`) (`GameplayStatics.GetWorldDeltaSeconds`))))))
    (:`then_2`
      ;[1 1 1] Rotate to cursor location
      (`SceneComponent.K2_SetWorldRotation` (`self.CapsuleComponent`) (`KismetMathLibrary.MakeRotator` _returnvalue_roll _returnvalue_pitch _returnvalue_yaw) false false))))

(fn `UserConstructionScript`)